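; BP_2ShadowMonster is a large shadow monster enemy that deals periodic damage to the player while they overlap it.
; Overlap by an actor of the player character's class starts a looping one-second timer, or unpauses the existing one, and ending the overlap pauses it.
; Each tick applies DamageAmount to player character 0 with the shadow monster damage type and the monster as causer.
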(event `self.ReceiveBeginPlay`)

(event `self.ReceiveActorBeginOverlap`
  (params (OtherActor :type "Actor Object Reference"))
  (if (== (`GameplayStatics.GetObjectClass` OtherActor) (`GameplayStatics.GetObjectClass` (`GameplayStatics.GetPlayerCharacter` 0)))
    (if (`KismetSystemLibrary.K2_TimerExistsHandle` (`self.DamagePlayerTimer`))
      (`KismetSystemLibrary.K2_UnPauseTimerHandle` (`self.DamagePlayerTimer`))
      (else
        (bind _returnvalue (`KismetSystemLibrary.K2_SetTimerDelegate` (delegate `Damage Player Over Time`) 1.0 true))
        (set `self.DamagePlayerTimer` _returnvalue)))))

(event `Damage Player Over Time`
  (`GameplayStatics.ApplyDamage` (`GameplayStatics.GetPlayerCharacter` 0) (`KismetMathLibrary.Conv_IntToDouble` (`self.Damage Amount`)) null self "/Game/4_Enemies/LargeShadowMonster/BP_ShadowMonster_DamageType.BP_ShadowMonster_DamageType_C"))

(event `self.ReceiveActorEndOverlap`
  (params (OtherActor :type "Actor Object Reference"))
  (if (== (`GameplayStatics.GetObjectClass` OtherActor) (`GameplayStatics.GetObjectClass` (`GameplayStatics.GetPlayerCharacter` 0)))
    (`KismetSystemLibrary.K2_PauseTimerHandle` (`self.DamagePlayerTimer`))))

(fn `UserConstructionScript`)