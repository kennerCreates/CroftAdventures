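; FlooringTile1_BP is a construction-time generator for a square floor of tiled static meshes.
; The construction script adds one static mesh component per cell of a Rows by Rows grid, using index modulo and division for X and Y.
; TileSize sets the spacing, with the grid centered on the actor's origin at zero height and each tile uniformly scaled up.
; The event graph holds no active logic.
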(fn `UserConstructionScript`
  (bind _rows (`self.Rows`))
  (for _index (range (* _rows _rows))
    (`AddComponent|NODE_AddStaticMeshComponent-0` :`RelativeTransform` (`KismetMathLibrary.MakeTransform` (`KismetMathLibrary.MakeVector` (`KismetMathLibrary.Conv_IntToDouble` (+ (- (* (mod _index (`self.Rows`)) (`self.TileSize`)) (/ (* (`self.Rows`) (`self.TileSize`)) 2)) (/ (`self.TileSize`) 2))) (`KismetMathLibrary.Conv_IntToDouble` (+ (- (* (/ _index (`self.Rows`)) (`self.TileSize`)) (/ (* (`self.Rows`) (`self.TileSize`)) 2)) (/ (`self.TileSize`) 2)))) (struct) (4.0 4.0 4.0)))))